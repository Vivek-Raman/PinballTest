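; BP_Bumper is a bumper that knocks BP_Ball actors away when they overlap it.
; On overlap it casts to the ball and applies a velocity-change impulse to its Ball component, pointing from the bumper's location toward the ball and scaled by BumperImpulse.
; The construction script assigns materials to the base and mechanism meshes.
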(event `self.ReceiveActorBeginOverlap`
  (params (OtherActor :type "Actor Object Reference"))
  (bind _asbp_ball (cast `/Game/Blueprints/BP_Ball` OtherActor))
  (`self.Bump` _asbp_ball))

(event `Bump`
  (params (Ball :type "/Game/Blueprints/BP_Ball Object Reference"))
  (`PrimitiveComponent.AddImpulse` (`/Game/Blueprints/BP_Ball.Ball` Ball) (* (`KismetMathLibrary.GetDirectionUnitVector` (`self.K2_GetActorLocation`) (`self.K2_GetActorLocation` Ball)) (`self.BumperImpulse`)) "None" true))

(fn `UserConstructionScript`
  (`PrimitiveComponent.SetMaterial` (`self.BumperBase`) 0 "/Game/Materials/M_BumperBase.M_BumperBase")
  (`PrimitiveComponent.SetMaterial` (`self.BumperMechanism`) 0 "/Game/Objects/M_Metal_Burnished_Steel.M_Metal_Burnished_Steel"))